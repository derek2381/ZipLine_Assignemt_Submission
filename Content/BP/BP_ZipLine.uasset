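; Zipline actor that strings a cable between Start and End sockets and reports a grab point to overlapping actors.
; The construction script places End and builds spline-mesh collision slightly below the line.
; On overlap, a timer estimates the point from horizontal distance to Start and sends it, both endpoints and Start's forward vector via an interface message.
; End overlap sends an empty message and clears timers; CheckDistance is an empty stub.
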(event `self.ReceiveBeginPlay`
  (bind _zipline_cable (`self.ZipLine Cable`))
  (bind _cablecollision (`self.CableCollision`))
  ;[1 1 1] Comment
  (`SceneComponent.K2_SetWorldLocation` _zipline_cable (`SceneComponent.GetSocketLocation` (`self.Start`) (`self.In Socket Name`)) false false)
  (`CableComponent.SetAttachEndToComponent` _zipline_cable (`self.End`) (`self.In Socket Name`))
  ;[1 1 1] Comment
  (add `PrimitiveComponent.OnComponentBeginOverlap` _cablecollision (delegate `On Player Detected`))
  (add `PrimitiveComponent.OnComponentEndOverlap` _cablecollision (delegate `Stop checking for Player`)))

(event `Stop checking for Player`
  (params (OverlappedComponent :type "PrimitiveComponent Object Reference") (OtherActor :type "Actor Object Reference") (OtherComp :type "PrimitiveComponent Object Reference") (OtherBodyIndex :type Integer))
  ;[1 1 1] Comment
  (message `/Game/BP/ZiplineInteract_BP.Interact Zipline` OtherActor false (0.0 0.0 0.0) (0.0 0.0 0.0) (0.0 0.0 0.0) (0.0 0.0 0.0))
  (`KismetSystemLibrary.K2_ClearAndInvalidateTimerHandle` (stale `On Player Detected` _returnvalue))
  (`KismetSystemLibrary.K2_ClearAndInvalidateTimerHandle` (stale `On Player Detected` _returnvalue_2)))

(event `On Player Detected`
  (params (OverlappedComponent :type "PrimitiveComponent Object Reference") (OtherActor :type "Actor Object Reference") (OtherComp :type "PrimitiveComponent Object Reference") (OtherBodyIndex :type Integer) (bFromSweep :type Boolean) (SweepResult :type "HitResult Structure (by ref)"))
  ;[1 1 1] Comment
  (bind _returnvalue (`KismetSystemLibrary.K2_SetTimerDelegate` (delegate `Set Current Target`) 0.05))
  (bind _returnvalue_2 (`KismetSystemLibrary.K2_SetTimerDelegate` (delegate `Check Distance`) 0.05)))

(event `Check Distance`
  ;[1 1 1] Comment
)

(event `Set Current Target`
  (bind (_startsocket _endsocket) (`self.Get Start and End Sockets`))
  ;[1 1 1] Comment
  (bind _output_get (set `self.Target Start Component` (`self.Find which zipline was interacted` (stale `On Player Detected` OtherActor))))
  (message `/Game/BP/ZiplineInteract_BP.Interact Zipline` (stale `On Player Detected` OtherActor) false _output_get _startsocket _endsocket (`SceneComponent.GetForwardVector` (`self.Start`))))

(fn `Find which zipline was interacted`
  (params (self2 :type "Actor Object Reference"))
  (returns (ReturnValue :type "Vector Structure"))
  (bind (_startsocket _endsocket) (`self.Get Start and End Sockets`))
  (bind (_returnvalue_x _returnvalue_y) (`KismetMathLibrary.BreakVector` (`self.K2_GetActorLocation` self2)))
  (bind (_returnvalue_x_2 _returnvalue_y_2) (`KismetMathLibrary.BreakVector` (`SceneComponent.GetSocketLocation` (`self.Start`) (`self.In Socket Name`))))
  (return (+ (* (`KismetMathLibrary.GetDirectionUnitVector` _startsocket _endsocket) (`KismetMathLibrary.VSize` (- (`KismetMathLibrary.MakeVector` _returnvalue_x _returnvalue_y) (`KismetMathLibrary.MakeVector` _returnvalue_x_2 _returnvalue_y_2)))) (`self.Get Start and End Sockets`))))

(fn `Get Start and End Sockets`
  (returns (StartSocket :type "Vector Structure") (EndSocket :type "Vector Structure"))
  (return (`SceneComponent.GetSocketLocation` (`self.Start`) (`self.In Socket Name`)) (`SceneComponent.GetSocketLocation` (`self.End`) (`self.In Socket Name`))))

(fn `UserConstructionScript`
  (bind _splinecollision (`self.SplineCollision`))
  (bind _splinecollision_2 (`self.SplineCollision`))
  (`SceneComponent.K2_SetRelativeLocation` (`self.End`) (`self.EndPoint`) false false)
  (`SplineComponent.SetLocationAtSplinePoint` (`self.SplineCollision`) 0 (`SceneComponent.GetSocketLocation` (`self.Start`) (`self.In Socket Name`)) "World" true)
  (`SplineComponent.SetLocationAtSplinePoint` (`self.SplineCollision`) 1 (`SceneComponent.GetSocketLocation` (`self.End`) "EndPoint") "World" true)
  (for _index (range (+ (- (`SplineComponent.GetNumberOfSplinePoints` (`self.SplineCollision`)) 2) 1))
    (bind _returnvalue (`AddComponent|NODE_AddSplineMeshComponent-0`))
    (set `self.CableCollision` _returnvalue)
    (bind _returnvalue_2 (+ _index 1))
    (`SplineMeshComponent.SetStartAndEnd` _returnvalue (- (`SplineComponent.GetLocationAtSplinePoint` _splinecollision _index "Local") (`KismetMathLibrary.MakeVector` 0.0 0.0 50.0)) (`SplineComponent.GetTangentAtSplinePoint` _splinecollision _index "Local") (- (`SplineComponent.GetLocationAtSplinePoint` _splinecollision_2 _returnvalue_2 "Local") (`KismetMathLibrary.MakeVector` 0.0 0.0 50.0)) (`SplineComponent.GetTangentAtSplinePoint` _splinecollision_2 _returnvalue_2 "Local") true)))